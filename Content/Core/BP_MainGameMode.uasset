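; Main game mode that sets up the HUD and owns the game's quest manager.
; On BeginPlay it creates WBP_MainDisplay for the first player controller, passes it the quest manager and adds it to the viewport.
; GetQuestManager lazily spawns a BP_QuestManager actor on first use and caches it for later calls.
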(event `self.ReceiveBeginPlay`
  ;[1 1 1] Main Game Mode Event
  (bind _returnvalue (`|CreateWidget` "/Game/UI/WBP_MainDisplay.WBP_MainDisplay_C" (`GameplayStatics.GetPlayerController` 0) (`self.GetQuestManager`)))
  (`UserWidget.AddToViewport` _returnvalue 0))

(fn `GetQuestManager`
  (returns (Output_Get :type "/Game/Quests/BP_QuestManager Object Reference"))
  ;[1 1 1] Quest Manager
  (`/Engine/EditorBlueprintResources/StandardMacros.IsValid` (`self.QuestManager`)
    (:`Is Valid`
      (return (`self.QuestManager`)))
    (:`Is Not Valid`
      (bind _returnvalue (`|SpawnActorFromClass` "/Game/Quests/BP_QuestManager.BP_QuestManager_C" (`KismetMathLibrary.MakeTransform` (0.0 0.0 0.0)) "Undefined" "OverrideRootScale" null null))
      (bind _output_get (set `self.QuestManager` _returnvalue))
      (return _output_get))))

(fn `UserConstructionScript`)