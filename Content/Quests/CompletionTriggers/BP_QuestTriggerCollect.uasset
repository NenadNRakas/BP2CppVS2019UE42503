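; Quest completion trigger that advances a quest when a tagged item enters its sphere collision volume.
; On sphere overlap, it checks the actor for the configured item tag and confirms it is not already in a seen-items list.
; Each new matching item is recorded, then the quest manager is told to complete the configured quest ID without completing the whole quest, so repeat overlaps by the same item are ignored.
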(event `self.Sphere.OnComponentBeginOverlap`
  (params (OverlappedComponent :type "PrimitiveComponent Object Reference") (OtherActor :type "Actor Object Reference") (OtherComp :type "PrimitiveComponent Object Reference") (OtherBodyIndex :type Integer) (bFromSweep :type Boolean) (SweepResult :type "HitResult Structure (by ref)"))
  ;[1 1 1] Collect Volume
  (if (and (`self.IsCorrectItem` OtherActor) (`self.HasNotSeenItem` OtherActor))
    (`self.MarkItemSeen` OtherActor)
    (`self.NotifyQuestComplete`)))

(fn `HasNotSeenItem`
  (params (ItemToFind :type "Actor Object Reference (by ref)"))
  (returns (ReturnValue :type Boolean))
  (return (not (`BlueprintSetLibrary.Set_Contains` (`self.SeenItems`) ItemToFind))))

(fn `IsCorrectItem`
  (params (Item :type "Actor Object Reference"))
  (returns (ReturnValue :type Boolean))
  (return (`self.ActorHasTag` Item (`self.ItemTag`))))

(fn `MarkItemSeen`
  (params (NewItem :type "Actor Object Reference (by ref)"))
  (`BlueprintSetLibrary.Set_Add` (`self.SeenItems`) NewItem))

(fn `NotifyQuestComplete`
  (`/Game/Quests/BP_QuestManager.CompleteQuest` (`/Game/Quests/BP_QuestLibrary.GetQuestManager`) (`self.QuestId`) false))

(fn `UserConstructionScript`)