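; BP_Grabber is a scene component that lets its owner pick up, carry and release physics objects.
; Grab sphere-traces forward for physics bodies, enables simulation on the hit component and attaches it at its center of mass to the owner's PhysicsHandle.
; Tick moves the handle target to a hold point ahead of the component.
; Grabbing also calls Pickup on any BP_QuestTriggerPickup component of the hit actor.
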(event `self.ReceiveTick`
  (params (DeltaSeconds :type "Float (single-precision)"))
  ;[1 1 1] Grabber Event Graph
  (`PhysicsHandleComponent.SetTargetLocationAndRotation` (`self.GetPhysicsComponent`) (`self.GetHoldLocation`) (`self.K2_GetComponentRotation`)))

(fn `GetHoldLocation`
  (returns (ReturnValue :type "Vector Structure"))
  (return (+ (`self.K2_GetComponentLocation`) (* (`KismetMathLibrary.GetForwardVector` (`self.K2_GetComponentRotation`)) (`self.HoldDistance`)))))

(fn `GetMaxGrabLocation`
  (returns (ReturnValue :type "Vector Structure"))
  ;[1 1 1] Max Grab Distance
  (return (+ (`self.K2_GetComponentLocation`) (* (`KismetMathLibrary.GetForwardVector` (`self.K2_GetComponentRotation`)) (`self.MaxGrabDistance`)))))

(fn `GetPhysicsComponent`
  (returns (ReturnValue :type "PhysicsHandleComponent Object Reference"))
  (return (`Actor.GetComponentByClass` (`self.GetOwner`) "/Script/Engine.PhysicsHandleComponent")))

(fn `Grab`
  ;[1 1 1] Grab Function
  (bind (_hitactor _hitcomponent _returnvalue) (`self.TraceForPhysicsBodies`))
  (if _returnvalue
    (`PrimitiveComponent.SetSimulatePhysics` _hitcomponent true) ; Some actors may not yet.
    (`PhysicsHandleComponent.GrabComponentAtLocationWithRotation` :`self` (`self.GetPhysicsComponent`) :`Component` _hitcomponent :`Location` (`PrimitiveComponent.GetCenterOfMass` _hitcomponent "None"))
    (`self.NotifyQuestActor` _hitactor)))

(fn `NotifyQuestActor`
  (params (Actor :type "Actor Object Reference"))
  (bind _returnvalue (`Actor.GetComponentByClass` Actor "/Game/Quests/CompletionTriggers/BP_QuestTriggerPickup.BP_QuestTriggerPickup_C"))
  ;[1 1 1] Grab
  (`/Engine/EditorBlueprintResources/StandardMacros.IsValid` _returnvalue
    (:`Is Valid`
      (`/Game/Quests/CompletionTriggers/BP_QuestTriggerPickup.Pickup` _returnvalue))))

(fn `Release`
  (`PhysicsHandleComponent.ReleaseComponent` (`self.GetPhysicsComponent`)))

(fn `TraceForPhysicsBodies`
  (returns (HitActor :type "Actor Object Reference") (HitComponent :type "PrimitiveComponent Object Reference") (ReturnValue :type Boolean))
  ;[1 1 1] Physics Trace for Bodies
  (bind (_outhit _returnvalue) (`KismetSystemLibrary.SphereTraceSingleForObjects` (`self.K2_GetComponentLocation`) (`self.GetMaxGrabLocation`) (`self.GrabRadius`) (`|MakeArray` "ObjectTypeQuery4" :!type "EObjectTypeQuery Enum")))
  (bind (_bblockinghit _binitialoverlap _time _distance _location _impactpoint _normal _impactnormal _physmat _hitactor _hitcomponent) (`GameplayStatics.BreakHitResult` _outhit))
  (return _hitactor _hitcomponent _returnvalue))